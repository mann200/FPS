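; Player controller for the multiplayer FPS deathmatch, linking each player to BP_DeathGame and the HUD.
; On death it reports the victim and killer to the game mode, destroys the pawn and requests a respawn.
; Spawn events create and possess the character, while client events handle input, timer, score data and the return to MainMenu.
; It creates the local UWB_PlayerUI and forwards ammo, health, score and recoil updates to it.
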(event `self.DeathMatchDeath`
  (params (DamageActor :type "Actor Object Reference"))
  ;[1 1 1] 玩家死亡相关
  (bind _asbp_death_game (cast `/Game/Blueprint/Game/Death/BP_DeathGame` (`GameplayStatics.GetGameMode`)))
  (`/Game/Blueprint/Game/Death/BP_DeathGame.SelfDeath` _asbp_death_game self)
  (bind _asbp_mulit_fpsplayer_controller (cast `/Game/Blueprint/Game/Death/BP_MulitFPSPlayerController` (`self.GetInstigatorController` DamageActor)))
  (`/Game/Blueprint/Game/Death/BP_DeathGame.KillAonther` _asbp_death_game _asbp_mulit_fpsplayer_controller)
  (`KismetSystemLibrary.Delay` 0.2)
  (`self.K2_DestroyActor` (`self.K2_GetPawn`))
  (bind _asbp_death_game_2 (cast `/Game/Blueprint/Game/Death/BP_DeathGame` (`GameplayStatics.GetGameMode`)))
  (`/Game/Blueprint/Game/Death/BP_DeathGame.RequestSpawn` _asbp_death_game_2 self))

(event `ClientDisableInput`
  ;[1 1 1] 玩家死亡相关
  (`self.DisableInput` (`self.K2_GetPawn`) self))

(event `ClientUpdataTime`
  (params (DelatTime :type Integer))
  (set `self.Time` DelatTime))

(event `ServerRequireUpdataValues`
  ;[1 1 1] 刷新数据
  (bind _asbp_death_game (cast `/Game/Blueprint/Game/Death/BP_DeathGame` (`GameplayStatics.GetGameMode`)))
  (`/Game/Blueprint/Game/Death/BP_DeathGame.UpdataValue` _asbp_death_game))

(event `ClientEndGame`
  (`GameplayStatics.OpenLevel` "MainMenu"))

(event `ClientUpdataValue`
  (params (Data :type "Array of DeathMacthPlayerData Structure"))
  ;[1 1 1] 刷新数据
  (bind _output_get (set `self.Data` Data))
  (`KismetMultiFPSLibrary.SortValues` _output_get)
  (bind _playerui (`self.PlayerUI`)
    (:`then`
      (`/Game/Blueprint/PlayerUI/DeathGame/UWB_PlayerUI.UpdataPlayerSroce` _playerui (`self.Data`)))
    (:`else`)))

(event `SpawnPlayerCharacter`
  (params (Class :type "/Game/Blueprint/Player/Death/BP_Attacker Class Reference") (SpawnTransform :type "Transform Structure"))
  (bind _returnvalue (`|SpawnActorFromClass` Class SpawnTransform "Undefined" "OverrideRootScale" null null))
  (`self.Possess` _returnvalue)
  (`self.ClientHideMouse`))

(event `ClientHideMouse`
  ;[1 1 1] 切换游戏模式
  (`WidgetBlueprintLibrary.SetInputMode_GameOnly` self)
  (set `self.bShowMouseCursor` false))

(event `self.CreatePlayerUI`
  ;[1 1 1] 基础设计
  (bind _playerui (`self.PlayerUI`)
    (:`then`
      (`Widget.RemoveFromParent` _playerui))
    (:`else`
      _))
  (if (`self.IsLocalPlayerController`)
    (bind _returnvalue (`|CreateWidget` "/Game/Blueprint/PlayerUI/DeathGame/UWB_PlayerUI.UWB_PlayerUI_C"))
    (bind _output_get (set `self.PlayerUI` _returnvalue))
    (`UserWidget.AddToViewport` _output_get 0)
    (`self.ServerRequireUpdataValues`)))

(event `self.DoRecoilAnim`
  ;[1 1 1] 基础设计
  (`/Game/Blueprint/PlayerUI/DeathGame/UWB_PlayerUI.DoRecoilAnim` (`self.PlayerUI`)))

(event `StartSpawnPlayer`
  (`KismetSystemLibrary.Delay` 1.0)
  (bind _asbp_death_game (cast `/Game/Blueprint/Game/Death/BP_DeathGame` (`GameplayStatics.GetGameMode`)))
  (`/Game/Blueprint/Game/Death/BP_DeathGame.RequestSpawn` _asbp_death_game self))

(event `self.UpdataPlayerAmmoUI`
  (params (ClipAmmo :type Integer) (GunCurrentAmmo :type Integer))
  ;[1 1 1] 基础设计
  (`/Game/Blueprint/PlayerUI/DeathGame/UWB_PlayerUI.UpdataAmmo` (`self.PlayerUI`) ClipAmmo GunCurrentAmmo))

(event `MyStartSpawnCharacter`
  (params (SpawnTransform :type "Transform Structure"))
  ;[1 1 1] 自已
  (`KismetSystemLibrary.Delay` 1.0)
  (bind _returnvalue (`|SpawnActorFromClass` "/Game/Blueprint/Player/Death/BP_Attacker.BP_Attacker_C" SpawnTransform "Undefined" "OverrideRootScale" null null))
  (`self.Possess` _returnvalue))

(event `self.UpdataPlayerHealthUI`
  (params (NewHealth :type "Float (single-precision)"))
  ;[1 1 1] 基础设计
  (`/Game/Blueprint/PlayerUI/DeathGame/UWB_PlayerUI.UpdataHealth` (`self.PlayerUI`) NewHealth))

(fn `UserConstructionScript`)