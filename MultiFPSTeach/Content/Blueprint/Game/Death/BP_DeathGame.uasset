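; Multiplayer FPS deathmatch game mode that manages player spawning, scoring and the match countdown.
; PostLogin registers each controller in a name/score map, and the first join caches PlayerStarts and starts a one-second looping timer.
; Kills add points and self-deaths subtract them, then scores are pushed to every client.
; RequestSpawn cycles BP_Attacker spawns through the start points, while the timer broadcasts remaining time and signals game end at zero.
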(event `self.K2_OnLogout`
  (params (ExitingController :type "Controller Object Reference")))

(event `KillAonther`
  (params (PlayerController :type "/Game/Blueprint/Game/Death/BP_MulitFPSPlayerController Object Reference"))
  (bind _playergamedatamap (`self.PlayerGameDataMap`))
  (bind (_playername _score) (break `DeathMacthPlayerData` (`BlueprintMapLibrary.Map_Find` (`self.PlayerGameDataMap`) PlayerController)))
  ;[1 1 1] 死亡相关（分数计算）
  (set `self.Player Name` _playername)
  (set `self.Score` _score)
  (`BlueprintMapLibrary.Map_Remove` _playergamedatamap PlayerController)
  (`BlueprintMapLibrary.Map_Add` _playergamedatamap PlayerController (make `DeathMacthPlayerData` (`self.Player Name`) (+ (`self.Score`) 15)))
  (`self.UpdataValue`))

(event `self.K2_PostLogin`
  (params (NewPlayer :type "PlayerController Object Reference"))
  ;[1 1 1] 玩家加入开始倒计时
  (if (not (`self.IsCharacterJoin`))
    (`self.GameStateSet`)
    (set `self.IsCharacterJoin` true))
  (bind _asbp_mulit_fpsplayer_controller (cast `/Game/Blueprint/Game/Death/BP_MulitFPSPlayerController` NewPlayer))
  (`/Game/Blueprint/Game/Death/BP_MulitFPSPlayerController.StartSpawnPlayer` _asbp_mulit_fpsplayer_controller)
  (`BlueprintMapLibrary.Map_Add` (`self.PlayerGameDataMap`) _asbp_mulit_fpsplayer_controller (make `DeathMacthPlayerData` (`KismetStringLibrary.Conv_StringToName` (`KismetSystemLibrary.GetObjectName` _asbp_mulit_fpsplayer_controller)))))

(event `SelfDeath`
  (params (PlayerController :type "/Game/Blueprint/Game/Death/BP_MulitFPSPlayerController Object Reference"))
  (bind _playergamedatamap (`self.PlayerGameDataMap`))
  (bind (_playername _score) (break `DeathMacthPlayerData` (`BlueprintMapLibrary.Map_Find` (`self.PlayerGameDataMap`) PlayerController)))
  ;[1 1 1] 死亡相关（分数计算）
  (set `self.Player Name` _playername)
  (set `self.Score` _score)
  (`BlueprintMapLibrary.Map_Remove` _playergamedatamap PlayerController)
  (`BlueprintMapLibrary.Map_Add` _playergamedatamap PlayerController (make `DeathMacthPlayerData` (`self.Player Name`) (- (`self.Score`) 10)))
  (`self.UpdataValue`))

(event `GameStateSet`
  ;[1 1 1] 玩家加入开始倒计时
  (bind _outactors (`GameplayStatics.GetAllActorsOfClass` "/Script/Engine.PlayerStart"))
  (set `self.CharacterSpawnPoints` _outactors)
  (bind _returnvalue (`KismetSystemLibrary.K2_SetTimerDelegate` (delegate `Down`) 1.0 true))
  (set `self.Timer` _returnvalue))

(event `UpdataValue`
  ;[1 1 1] 排行榜更新
  (bind _keys (`BlueprintMapLibrary.Map_Keys` (`self.PlayerGameDataMap`)))
  (for _array_element _keys
    (bind _values (`BlueprintMapLibrary.Map_Values` (`self.PlayerGameDataMap`)))
    (`/Game/Blueprint/Game/Death/BP_MulitFPSPlayerController.ClientUpdataValue` _array_element _values)))

(event `Down`
  ;[1 1 1] 玩家加入开始倒计时
  (set `self.Time` (- (`self.Time`) 1))
  (bind _keys (`BlueprintMapLibrary.Map_Keys` (`self.PlayerGameDataMap`)))
  (for _array_element _keys
    (`/Game/Blueprint/Game/Death/BP_MulitFPSPlayerController.ClientUpdataTime` _array_element (`self.Time`)))
  (if (<= (`self.Time`) 0)
    (bind _keys_2 (`BlueprintMapLibrary.Map_Keys` (`self.PlayerGameDataMap`)))
    (for _array_element_2 _keys_2
      (`/Game/Blueprint/Game/Death/BP_MulitFPSPlayerController.ClientEndGame` _array_element_2))))

(event `RequestSpawn`
  (params (PlayerControl :type "/Game/Blueprint/Game/Death/BP_MulitFPSPlayerController Object Reference"))
  (bind _characterspawnpoints (`self.CharacterSpawnPoints`))
  ;[1 1 1] 玩家位置
  (`/Game/Blueprint/Game/Death/BP_MulitFPSPlayerController.SpawnPlayerCharacter` PlayerControl "/Game/Blueprint/Player/Death/BP_Attacker.BP_Attacker_C" (`self.GetTransform` (`|GetArrayItem` _characterspawnpoints (`self.SpawnPointIndex`))))
  (bind _output_get (set `self.SpawnPointIndex` (+ (`self.SpawnPointIndex`) 1)))
  (if (> _output_get (- (`KismetArrayLibrary.Array_Length` _characterspawnpoints) 1))
    (set `self.SpawnPointIndex` 0)))

(fn `UserConstructionScript`)