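; Game mode for a round-based 5v5 Police vs Kidnapper match that alternates joining players between teams and spawns them at tagged PlayerStarts.
; A per-controller map tracks money, kills and deaths and pushes updates to every controller alongside round and clock state.
; A one-second timer and team death counts end rounds, with timeouts going to Police.
; Matches end past half the rounds with a two-win lead; the explode outcome is stubbed.
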(event `self.ReceiveBeginPlay`
  (`|ExecutionSequence`
    (:`then_0`
      (bind _outactors (`GameplayStatics.GetAllActorsOfClass` "/Script/Engine.PlayerStart"))
      (for _array_element _outactors
        (switch `name` (`PlayerStart.PlayerStartTag` _array_element)
          (:`Police`
            (`KismetArrayLibrary.Array_Add` (`self.PolicePointArray`) _array_element))
          (:`Kidnapper`
            (`KismetArrayLibrary.Array_Add` (`self.KidnapperPointArray`) _array_element)))))))

(event `CheckGameRule`
  (params (Player :type "/Game/Blueprint/Game/5V5/BP_5V5PlayerControl Object Reference"))
  ;[1 1 1] 检测游戏规则
  (switch `/Game/Blueprint/Player/5v5/Enum_TeamType` (`/Game/Blueprint/Game/5V5/BP_5V5PlayerControl.TeamType` Player)
    (:`NewEnumerator0`
      (bind _result (`/Engine/EditorBlueprintResources/StandardMacros.IncrementInt` (`self.PoliceDeathNum`))
        (:`  `
          (set `self.PoliceDeathNum` _result)
          (if (>= (`self.PoliceDeathNum`) (`KismetArrayLibrary.Array_Length` (`self.PoliceTeam`)))
            (set `self.PoliceDeathNum` 0)
            (`self.NewGameRound` "NewEnumerator0" "NewEnumerator1")))))
    (:`NewEnumerator1`
      (bind _result_2 (`/Engine/EditorBlueprintResources/StandardMacros.IncrementInt` (`self.KidnapperDeathNum`))
        (:`  `
          (set `self.KidnapperDeathNum` _result_2)
          (if (>= (`self.KidnapperDeathNum`) (`KismetArrayLibrary.Array_Length` (`self.KidnapperTeam`)))
            (set `self.PoliceDeathNum` 0)
            (`self.NewGameRound` "NewEnumerator0")))))))

(event `self.K2_OnLogout`
  (params (ExitingController :type "Controller Object Reference")))

(event `SelfDeath`
  (params (Player :type "/Game/Blueprint/Game/5V5/BP_5V5PlayerControl Object Reference"))
  (bind (_money _kill _death _assist) (break `/Game/Blueprint/Player/5v5/S_PlayerState` (`self.OldPlayerState`)))
  (bind (_value _returnvalue) (`BlueprintMapLibrary.Map_Find` (`self.AllPlayerState`) Player))
  ;[1 1 1] 自身死亡调用
  (bind _output_get (set `self.DeathPlayer` Player))
  (`self.K2_DestroyActor` (`Controller.K2_GetPawn` _output_get))
  (if _returnvalue
    (set `self.OldPlayerState` _value)
    (`BlueprintMapLibrary.Map_Remove` (`self.AllPlayerState`) (`self.DeathPlayer`))
    (`BlueprintMapLibrary.Map_Add` (`self.AllPlayerState`) (`self.DeathPlayer`) (make `/Game/Blueprint/Player/5v5/S_PlayerState` _money _kill (+ _death 1) _assist))
    (`self.UpdataPlayerState`)
    (`self.CheckGameRule` (`self.DeathPlayer`))))

(event `self.K2_PostLogin`
  (params (NewPlayer :type "PlayerController Object Reference"))
  ;[1 1 1] 玩家登录房间
  (bind _asbp_5v5player_control (cast `/Game/Blueprint/Game/5V5/BP_5V5PlayerControl` NewPlayer))
  (set `self.NewPlayer` _asbp_5v5player_control)
  (bind _output_get (set `self.PlayerNum` (+ (`self.PlayerNum`) 1)))
  (if (== (mod _output_get 2) 0)
    (bind _returnvalue (`KismetArrayLibrary.Array_Add` (`self.KidnapperTeam`) (`self.NewPlayer`)))
    (set `self.Sequence` _returnvalue)
    (set `self.Team Type` "NewEnumerator1")
    (`BlueprintMapLibrary.Map_Add` (`self.AllPlayerState`) (`self.NewPlayer`) (`self.InitPlayerState`))
    (`/Game/Blueprint/Game/5V5/BP_5V5PlayerControl.StartSpawnPlayer` (`self.NewPlayer`) (`self.Sequence`) (`self.Team Type`) (`self.KidnapperTeam`))
    (`self.UpdataGameState`)
    (if (`self.NewVar_0`)
      (set `self.NewVar_0` false)
      (`KismetSystemLibrary.Delay` 1.0)
      (`self.GameStart`))
    (else
      (bind _returnvalue_2 (`KismetArrayLibrary.Array_Add` (`self.PoliceTeam`) (`self.NewPlayer`)))
      (set `self.Sequence` _returnvalue_2)
      (set `self.Team Type` "NewEnumerator0")
      (`BlueprintMapLibrary.Map_Add` (`self.AllPlayerState`) (`self.NewPlayer`) (`self.InitPlayerState`))
      (`/Game/Blueprint/Game/5V5/BP_5V5PlayerControl.StartSpawnPlayer` (`self.NewPlayer`) (`self.Sequence`) (`self.Team Type`) (`self.PoliceTeam`))
      (`self.UpdataGameState`))))

(event `KillOther`
  (params (Player :type "/Game/Blueprint/Game/5V5/BP_5V5PlayerControl Object Reference"))
  (bind _allplayerstate (`self.AllPlayerState`))
  (bind (_money _kill _death _assist) (break `/Game/Blueprint/Player/5v5/S_PlayerState` (`self.OldPlayerState`)))
  (bind (_value _returnvalue) (`BlueprintMapLibrary.Map_Find` _allplayerstate Player))
  ;[1 1 1] 击杀敌人调用
  (if _returnvalue
    (set `self.OldPlayerState` _value)
    (`BlueprintMapLibrary.Map_Remove` _allplayerstate Player)
    (`BlueprintMapLibrary.Map_Add` _allplayerstate Player (make `/Game/Blueprint/Player/5v5/S_PlayerState` (+ _money 2000) (+ _kill 1) _death _assist))
    (`self.UpdataPlayerState`)
    (else
      (`KismetSystemLibrary.PrintString` "Hello"))))

(event `UpdataPlayerState`
  (bind _allplayerstate (`self.AllPlayerState`))
  ;[1 1 1] 更新玩家数据
  (bind _keys (`BlueprintMapLibrary.Map_Keys` _allplayerstate))
  (for _array_element _keys
    (bind (_value _returnvalue) (`BlueprintMapLibrary.Map_Find` _allplayerstate _array_element))
    (if _returnvalue
      (`/Game/Blueprint/Game/5V5/BP_5V5PlayerControl.UpdataPlayerState` _array_element _value))))

(event `GameStart`
  ;[1 1 1] 游戏规则
  (bind _returnvalue (`KismetSystemLibrary.K2_SetTimerDelegate` (delegate `GameRule`) 1.0 true))
  (set `self.Timer` _returnvalue))

(event `UpdataGameState`
  ;[1 1 1] 更新游戏数据
  (bind _keys (`BlueprintMapLibrary.Map_Keys` (`self.AllPlayerState`)))
  (for _array_element _keys
    (`/Game/Blueprint/Game/5V5/BP_5V5PlayerControl.UpdataGameState` _array_element (`self.PoliceWinRounds`) (`self.KidnapperWinRounds`) (`self.CurrentRound`) (`self.TotalRounds`) (`self.Time_Minute`) (`self.Time_Seconds`))))

(event `BuyArmor`
  (params (Player :type "/Game/Blueprint/Game/5V5/BP_5V5PlayerControl Object Reference") (bHead :type Boolean) (Money :type Integer))
  (`/Game/Blueprint/Game/5V5/BP_5V5PlayerControl.RequestBuyArmor` Player bHead Money))

(event `GameRule`
  (bind _returnvalue (- (`self.Time_Seconds`) 1))
  (bind _returnvalue_2 (- (`self.Time_Minute`) 1))
  ;[1 1 1] 游戏规则
  (if (< _returnvalue 0)
    (if (< _returnvalue_2 0)
      (`KismetSystemLibrary.Delay` 1.0)
      (`self.NewGameRound` "NewEnumerator1")
      (else
        (set `self.Time_Minute` _returnvalue_2)
        (set `self.Time_Seconds` 59)
        (`self.UpdataGameState`)))
    (else
      (set `self.Time_Seconds` _returnvalue)
      (`self.UpdataGameState`))))

(event `RequestSpawn`
  (params (PlayerControl :type "/Game/Blueprint/Game/5V5/BP_5V5PlayerControl Object Reference") (Sequence :type Integer) (TeamType :type "/Game/Blueprint/Player/5v5/Enum_TeamType Enum" :default "NewEnumerator0"))
  ;[1 1 1] 生成角色
  (switch `/Game/Blueprint/Player/5v5/Enum_TeamType` TeamType
    (:`NewEnumerator0`
      (set `self.CurrentPoint` (`|GetArrayItem` (`self.PolicePointArray`) Sequence)))
    (:`NewEnumerator1`
      (set `self.CurrentPoint` (`|GetArrayItem` (`self.KidnapperPointArray`) Sequence))))
  (`/Game/Blueprint/Game/5V5/BP_5V5PlayerControl.SpawnPlayerCharacter` PlayerControl "/Game/Blueprint/Player/5v5/BP_5V5PlayerCharacter.BP_5V5PlayerCharacter_C" (`self.GetTransform` (`self.CurrentPoint`)))
  (`self.UpdataPlayerState`))

(event `NewGameRound`
  (params (GameRule :type "/Game/Blueprint/Player/5v5/Enum_GameRule Enum" :default "NewEnumerator0") (TeamType :type "/Game/Blueprint/Player/5v5/Enum_TeamType Enum" :default "NewEnumerator0"))
  ;[1 1 1] 游戏规则
  (`KismetSystemLibrary.K2_PauseTimerHandle` (`self.Timer`))
  (switch `/Game/Blueprint/Player/5v5/Enum_GameRule` GameRule
    (:`NewEnumerator0`
      (`self.Defeat` TeamType))
    (:`NewEnumerator1`
      (`self.TimeOver`))
    (:`NewEnumerator2`
      (`self.Explpde`)))
  (`KismetSystemLibrary.K2_UnPauseTimerHandle` (`self.Timer`))
  (bind _keys (`BlueprintMapLibrary.Map_Keys` (`self.AllPlayerState`)))
  (for _array_element _keys
    (`/Game/Blueprint/Game/5V5/BP_5V5PlayerControl.Rebirth` _array_element))
  (`self.UpdataGameState`))

(fn `Defeat`
  (params (GameTeam :type "/Game/Blueprint/Player/5v5/Enum_TeamType Enum" :default "NewEnumerator0"))
  (switch `/Game/Blueprint/Player/5v5/Enum_TeamType` GameTeam
    (:`NewEnumerator0`
      (bind _result (`/Engine/EditorBlueprintResources/StandardMacros.IncrementInt` (`self.PoliceWinRounds`))
        (:`  `
          (set `self.PoliceWinRounds` _result))))
    (:`NewEnumerator1`
      (bind _result_2 (`/Engine/EditorBlueprintResources/StandardMacros.IncrementInt` (`self.KidnapperWinRounds`))
        (:`  `
          (set `self.KidnapperWinRounds` _result_2)))))
  (if (`self.RoundCount`)
    (bind _keys (`BlueprintMapLibrary.Map_Keys` (`self.AllPlayerState`)))
    (for _array_element _keys
      (switch `/Game/Blueprint/Player/5v5/Enum_TeamType` (`/Game/Blueprint/Game/5V5/BP_5V5PlayerControl.TeamType` _array_element)
        (:`NewEnumerator0`
          (`/Game/Blueprint/Game/5V5/BP_5V5PlayerControl.GameEnd` _array_element (select `bool` (> (`self.PoliceWinRounds`) (`self.KidnapperWinRounds`)) :`false` "你输了！" :`true` "你赢了！" :!type "Text")))
        (:`NewEnumerator1`
          (`/Game/Blueprint/Game/5V5/BP_5V5PlayerControl.GameEnd` _array_element (select `bool` (> (`self.KidnapperWinRounds`) (`self.PoliceWinRounds`)) :`false` "你输了！" :`true` "你赢了！" :!type "Text")))))
    (else
      (set `self.Time_Minute` 3)
      (set `self.Time_Seconds` 0))))

(fn `Explpde`)

(fn `InPlayerTypeSet`
  (params (Player :type "/Game/Blueprint/Game/5V5/BP_5V5PlayerControl Object Reference"))
  (bind _output_get (set `self.PlayerNum` (+ (`self.PlayerNum`) 1))))

(fn `RoundCount`
  (returns (ReturnValue :type Boolean))
  (bind _result (`/Engine/EditorBlueprintResources/StandardMacros.IncrementInt` (`self.CurrentRound`))
    (:`  `
      (bind _output_get (set `self.CurrentRound` _result))
      (return (and (> _output_get (/ (`self.TotalRounds`) 2)) (or (>= (`self.PoliceWinRounds`) (+ (`self.KidnapperWinRounds`) 2)) (>= (`self.KidnapperWinRounds`) (+ (`self.PoliceWinRounds`) 2))))))))

(fn `TimeOver`
  (bind _result (`/Engine/EditorBlueprintResources/StandardMacros.IncrementInt` (`self.PoliceWinRounds`))
    (:`  `
      (set `self.PoliceWinRounds` _result)
      (if (`self.RoundCount`)
        (`KismetSystemLibrary.PrintString` "Game End" true true (struct :`R` 1.0 :`B` 0.038797 :`A` 1.0) 20.0)
        (else
          (set `self.Time_Minute` 3)
          (set `self.Time_Seconds` 0))))))

(fn `UserConstructionScript`)