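; Player controller for a round-based 5v5 Police-versus-Kidnapper shooter, managing each player's pawn, economy and UI.
; It spawns, possesses and resets the character with cached armor, and forwards weapon switches and purchases to it.
; Spawn requests, death and kill reports, and scoreboard team data go through BP_5V5GM.
; It owns the HUD, Tab scoreboard, B-key shop and game-end screen, switching input modes and caching player and round state.
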(event `SpawnPlayerCharacter`
  (params (Class :type "/Game/Blueprint/Player/5v5/BP_5V5PlayerCharacter Class Reference") (SpawnTransform :type "Transform Structure"))
  ;[1 1 1] 开始生成角色
  (bind _output_get (set `self.PlayerClass` Class))
  (bind _output_get_2 (set `self.Spawn Transform` SpawnTransform))
  (bind _returnvalue (`|SpawnActorFromClass` _output_get _output_get_2 "Undefined" "OverrideRootScale" self null))
  (bind _output_get_3 (set `self.5v5Character` _returnvalue))
  (`self.Possess` _output_get_3)
  (`self.ClientHideMouse`))

(event `ClientHideMouse`
  ;[1 1 1] 切换游戏模式
  (`WidgetBlueprintLibrary.SetInputMode_GameOnly` self)
  (set `self.bShowMouseCursor` false))

(event `self.CreatePlayerUI`
  ;[1 1 1] 基础设计
  (bind _playerui (`self.PlayerUI`)
    (:`then`
      (`Widget.RemoveFromParent` _playerui))
    (:`else`
      _))
  (if (`self.IsLocalPlayerController`)
    (bind _returnvalue (`|CreateWidget` "/Game/Blueprint/PlayerUI/5V5/WB_5V5MainUI.WB_5V5MainUI_C"))
    (bind _output_get (set `self.PlayerUI` _returnvalue))
    (`UserWidget.AddToViewport` _output_get 0)
    (set `/Game/Blueprint/PlayerUI/5V5/WB_5V5MainUI.Player` self _output_get)))

(event `ClientShowMouse`
  ;[1 1 1] 切换游戏模式
  (`WidgetBlueprintLibrary.SetInputMode_GameAndUIEx` self null)
  (set `self.bShowMouseCursor` true))

(event `StartSpawnPlayer`
  (params (Sequence :type Integer) (TeamType :type "/Game/Blueprint/Player/5v5/Enum_TeamType Enum" :default "NewEnumerator0") (Team :type "Array of /Game/Blueprint/Game/5V5/BP_5V5PlayerControl Object Reference"))
  ;[1 1 1] 开始生成角色
  (`KismetSystemLibrary.Delay` 1.0)
  (bind _asbp_5v5gm (cast `/Game/Blueprint/Game/5V5/BP_5V5GM` (`GameplayStatics.GetGameMode`)))
  (`/Game/Blueprint/Game/5V5/BP_5V5GM.RequestSpawn` _asbp_5v5gm self Sequence TeamType)
  (set `self.Team` Team)
  (set `self.TeamType` TeamType))

(event `self.DoRecoilAnim`
  ;[1 1 1] 基础设计
  (`/Game/Blueprint/PlayerUI/5V5/WB_5V5MainUI.DoRecoilAnim` (`self.PlayerUI`)))

(event `self.UpdataPlayerAmmoUI`
  (params (ClipAmmo :type Integer) (GunCurrentAmmo :type Integer))
  ;[1 1 1] 基础设计
  (`/Game/Blueprint/PlayerUI/5V5/WB_5V5MainUI.UpdataAmmo` (`self.PlayerUI`) ClipAmmo GunCurrentAmmo))

(event `Key|Tab`
  (params (Key :type "Key Structure"))
  ;[1 1 1] 统计表
  (:`Pressed`
    (bind _dataui (`self.DataUI`)
      (:`then`
        (`Widget.RemoveFromParent` _dataui)
        (set `self.DataUI` null))
      (:`else`
        (`self.CreateDataUINotify`)))))

(event `Rebirth`
  (bind _5v5character (`self.5v5Character`))
  ;[1 1 1] 重置位置
  (`/Engine/EditorBlueprintResources/StandardMacros.IsValid` (`self.5v5Character`)
    (:`Is Valid`
      (`self.K2_SetActorTransform` _5v5character (`self.Spawn Transform`) false false)
      (`self.Possess` _5v5character)
      (`FPSTeachBaseCharacter.ReSetPlayerState` (`self.5v5Character`) 100.0 (`self.Head Armor`) (`self.Body Armor`)))
    (:`Is Not Valid`
      (bind _returnvalue (`|SpawnActorFromClass` (`self.PlayerClass`) (`self.Spawn Transform`) "Undefined" "OverrideRootScale" self null))
      (bind _output_get (set `self.5v5Character` _returnvalue))
      (`self.Possess` _output_get)
      (`FPSTeachBaseCharacter.ReSetPlayerState` (`self.5v5Character`) 100.0 (`self.Head Armor`) (`self.Body Armor`)))))

(event `self.UpdataPlayerHealthUI`
  (params (NewHealth :type "Float (single-precision)") (NewHeadArmor :type "Float (single-precision)") (NewBodyArmor :type "Float (single-precision)"))
  ;[1 1 1] 基础设计
  (`/Game/Blueprint/PlayerUI/5V5/WB_5V5MainUI.UpdataHealth` (`self.PlayerUI`) NewHealth NewHeadArmor NewBodyArmor)
  (set `self.Head Armor` NewHeadArmor)
  (set `self.Body Armor` NewBodyArmor))

(event `CreateDataUINotify`
  ;[1 1 1] 统计表
  (bind _asbp_5v5gm (cast `/Game/Blueprint/Game/5V5/BP_5V5GM` (`GameplayStatics.GetGameMode`)))
  (`self.ClientCreateDataUI` (`/Game/Blueprint/Game/5V5/BP_5V5GM.PoliceTeam` _asbp_5v5gm) (`/Game/Blueprint/Game/5V5/BP_5V5GM.KidnapperTeam` _asbp_5v5gm)))

(event `self.DeathMatchDeath`
  (params (DamageActor :type "Actor Object Reference"))
  ;[1 1 1] 死亡相关
  (bind _asbp_5v5gm (cast `/Game/Blueprint/Game/5V5/BP_5V5GM` (`GameplayStatics.GetGameMode`)))
  (bind _asbp_5v5player_control (cast `/Game/Blueprint/Game/5V5/BP_5V5PlayerControl` (`self.GetInstigatorController` DamageActor)))
  (`/Game/Blueprint/Game/5V5/BP_5V5GM.SelfDeath` _asbp_5v5gm self)
  (`/Game/Blueprint/Game/5V5/BP_5V5GM.KillOther` _asbp_5v5gm _asbp_5v5player_control))

(event `ClientCreateDataUI`
  (params (Police :type "Array of /Game/Blueprint/Game/5V5/BP_5V5PlayerControl Object Reference (by ref)") (Kidnapper :type "Array of /Game/Blueprint/Game/5V5/BP_5V5PlayerControl Object Reference (by ref)"))
  ;[1 1 1] 统计表
  (bind _returnvalue (`|CreateWidget` "/Game/Blueprint/PlayerUI/5V5/WB_5V5Data.WB_5V5Data_C" self))
  (bind _output_get (set `self.DataUI` _returnvalue))
  (`UserWidget.AddToViewport` _output_get 0)
  (`/Game/Blueprint/PlayerUI/5V5/WB_5V5Data.UpdataPlayerSroce` _output_get Police Kidnapper))

(event `GameEnd`
  (params (GameText :type Text))
  (bind _returnvalue (`|CreateWidget` "/Game/Blueprint/PlayerUI/5V5/WB_GameEnd.WB_GameEnd_C" self))
  (`UserWidget.AddToViewport` _returnvalue 0)
  (set `/Game/Blueprint/PlayerUI/5V5/WB_GameEnd.GameText` GameText _returnvalue)
  (`WidgetBlueprintLibrary.SetInputMode_UIOnlyEx` self null)
  (set `self.bShowMouseCursor` true))

(event `BuyWeapon`
  (params (WeaponType :type "EWeaponType Enum" :default "AK47") (Money :type Integer))
  (bind _money (`self.Money`))
  ;[1 1 1] C++（已经在服务器运行）
  (if (<= Money _money)
    (set `self.Money` (- _money Money))
    (`FPSTeachBaseCharacter.BuyWeaponFun` (`self.5v5Character`) WeaponType)))

(event `ResponseBuyArmor`
  (params (bHead :type Boolean) (money :type Integer))
  ;[1 1 1] C++（已经在服务器运行）
  (bind _asbp_5v5gm (cast `/Game/Blueprint/Game/5V5/BP_5V5GM` (`GameplayStatics.GetGameMode`)))
  (`/Game/Blueprint/Game/5V5/BP_5V5GM.BuyArmor` _asbp_5v5gm self bHead money))

(event `Key|One`
  (params (Key :type "Key Structure"))
  ;[1 1 1] 切换武器
  (:`Pressed`
    (`self.SwitchWeapon` "PrimaryWeapon")))

(event `Key|Three`
  (params (Key :type "Key Structure"))
  ;[1 1 1] 切换武器
  (:`Pressed`
    (`self.SwitchWeapon` "Knife")))

(event `SwitchWeapon`
  (params (SwitchType :type "EWeapon Enum" :default "PrimaryWeapon"))
  ;[1 1 1] C++（已经在服务器运行）
  (`FPSTeachBaseCharacter.SwitchWeaponFun` (`self.5v5Character`) SwitchType))

(event `RequestBuyArmor`
  (params (bHead :type Boolean) (Money :type Integer))
  (bind _money (`self.Money`))
  ;[1 1 1] C++（已经在服务器运行）
  (if (<= Money _money)
    (set `self.Money` (- _money Money))
    (if true
      (set `self.Head Armor` 100.0)
      (else
        (set `self.Body Armor` 100.0)))
    ;;[1 1 1] 服务器无法更新，待解决
    (`FPSTeachBaseCharacter.BuyArmor` (`self.5v5Character`) bHead)))

(event `Key|Two`
  (params (Key :type "Key Structure"))
  ;[1 1 1] 切换武器
  (:`Pressed`
    (`self.SwitchWeapon` "SecondaryWeapans")))

(event `Key|B`
  (params (Key :type "Key Structure"))
  ;[1 1 1] 商店
  (:`Pressed`
    (bind _shopui (`self.ShopUI`)
      (:`then`
        (`Widget.RemoveFromParent` _shopui)
        (set `self.ShopUI` null)
        (`self.ClientHideMouse`))
      (:`else`
        (bind _returnvalue (`|CreateWidget` "/Game/Blueprint/PlayerUI/5V5/WB_Shop.WB_Shop_C"))
        (set `self.ShopUI` _returnvalue)
        (set `/Game/Blueprint/PlayerUI/5V5/WB_Shop.Player` self _returnvalue)
        (set `/Game/Blueprint/PlayerUI/5V5/WB_Shop.Team` (`self.Team`) _returnvalue)
        (`UserWidget.AddToViewport` _returnvalue 0)
        (`self.ClientShowMouse`)))))

(fn `UpdataGameState`
  (params (PoliceWinRound :type Integer) (KidnapperWinRound :type Integer) (CurrentRound :type Integer) (TotalRounds :type Integer) (Time_Minute :type Integer) (Time_Seconds :type Integer))
  (set `self.PoliceWinRound` PoliceWinRound)
  (set `self.KidnapperWinRound` KidnapperWinRound)
  (set `self.CurrentRound` CurrentRound)
  (set `self.TotalRounds` TotalRounds)
  (set `self.Time_Minute` Time_Minute)
  (set `self.Time_Seconds` Time_Seconds))

(fn `UpdataPlayerState`
  (params (State :type "/Game/Blueprint/Player/5v5/S_PlayerState Structure"))
  (bind (_money _kill _death _assist) (break `/Game/Blueprint/Player/5v5/S_PlayerState` State))
  (set `self.Money` _money)
  (set `self.Kill` _kill)
  (set `self.Death` _death)
  (set `self.Assist` _assist))

(fn `UserConstructionScript`)