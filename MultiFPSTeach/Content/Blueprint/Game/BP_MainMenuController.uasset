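; Main menu player controller that shows the menu widgets and hosts multiplayer sessions.
; BeginPlay adds UWB_Main with the cursor visible, and OpenUI swaps it for a fresh UWB_MainMenuUI in UI-only input.
; CreateSession destroys any old session, then on either result creates an Advanced Session using DataSettings' game type, map and match properties.
; Success opens the mode's level as a listen server, although the session is flagged dedicated.
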(event `self.ReceiveBeginPlay`
  (bind _returnvalue (`|CreateWidget` "/Game/Blueprint/PlayerUI/StartUI/UWB_Main.UWB_Main_C" self))
  (bind _output_get (set `self.Main` _returnvalue))
  (`UserWidget.AddToViewport` _output_get 0)
  (set `self.bShowMouseCursor` true))

(event `OpenUI`
  (bind _mainmenuui (`self.MainMenuUI`))
  (`Widget.RemoveFromParent` (`self.Main`))
  (`/Engine/EditorBlueprintResources/StandardMacros.IsValid` _mainmenuui
    (:`Is Valid`
      (`Widget.RemoveFromParent` _mainmenuui))
    (:`Is Not Valid`
      _))
  (bind _returnvalue (`|CreateWidget` "/Game/Blueprint/PlayerUI/StartUI/UWB_MainMenuUI.UWB_MainMenuUI_C"))
  (bind _output_get (set `self.MainMenuUI` _returnvalue))
  (`UserWidget.AddToViewport` _output_get 0)
  (`WidgetBlueprintLibrary.SetInputMode_UIOnlyEx` self null))

(event `CreateSession`
  (params (GameType :type String) (MapName :type "EditableTextBox Object Reference") (bUseLAN :type Boolean) (PublicConnections :type Integer))
  (set `self.Game Type` GameType)
  (`DestroySessionCallbackProxy.DestroySession` self self
    (:`OnSuccess`
      _)
    (:`OnFailure`
      _))
  (bind _settings (`self.DataSettings` MapName))
  (`CreateSessionCallbackProxyAdvanced.CreateAdvancedSession` _settings self PublicConnections 0 bUseLAN true true false
    (:`then`
      (`KismetSystemLibrary.PrintString` "房间正在创建" true true (struct :`R` 1.0 :`B` 0.085174 :`A` 1.0) 10.0))
    (:`OnSuccess`
      (switch `string` (`self.Game Type`)
        (:`死亡竞速`
          (`GameplayStatics.OpenLevel` "DeathMap" true "Listen"))
        (:`5v5竞技`
          (`GameplayStatics.OpenLevel` "5v5Level" true "Listen"))))
    (:`OnFailure`
      (`KismetSystemLibrary.PrintString` "房间创建失败" true true (struct :`R` 1.0 :`B` 0.085174 :`A` 1.0) 10.0))))

(fn `DataSettings`
  (params (MapName :type "EditableTextBox Object Reference"))
  (returns (Settings :type "Array of SessionPropertyKeyPair Structure"))
  (return (`|MakeArray` (`AdvancedSessionsLibrary.MakeLiteralSessionPropertyString` "GameType" (`self.Game Type`)) (`AdvancedSessionsLibrary.MakeLiteralSessionPropertyInt` "PlayerNums") (`AdvancedSessionsLibrary.MakeLiteralSessionPropertyString` "MapName" (`KismetTextLibrary.Conv_TextToString` (`EditableTextBox.GetText` MapName))) (`AdvancedSessionsLibrary.MakeLiteralSessionPropertyInt` "Bout" 10))))

(fn `UserConstructionScript`)